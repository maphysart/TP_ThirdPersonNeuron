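; Network controller actor that connects to a Neuron motion data stream (BVH skeleton motion) at a configurable host and port.
; On BeginPlay it initializes from a BVH reference file or from defaults with a hips bone offset, then connects if that succeeds.
; A reconnect event drops and reopens the connection behind a re-entry blocker flag, and both connection paths store the result in NeuronConnected.
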(event `self.ReceiveBeginPlay`
  ;[1 1 1] On BeginPlay Init Neuron Controller and connect
  (if (`self.InitWithBVHReferenceFile`)
    (bind _returnvalue (`PerceptionNeuronBPLibrary.NeuronInitFile` self (`self.ReferenceSkeletonFileName`) (`self.Motion Line Format`)))
    (if _returnvalue
      (bind _returnvalue_2 (`PerceptionNeuronBPLibrary.NeuronConnect` self (`self.HostName`) (`self.Port`) (`self.EnableReferenceBone`) (`self.EnableDisplacement`) (`self.Motion Line Format`) :!label _label))
      (set `self.NeuronConnected` _returnvalue_2))
    (else
      (bind _returnvalue_3 (`PerceptionNeuronBPLibrary.NeuronInit` self))
      (if _returnvalue_3
        (bind _returnvalue_4 (`PerceptionNeuronBPLibrary.NeuronBoneSetOffset` self 0 0.0 95.32)) ; Set Hips Bone Offset
        (if _returnvalue_4
          (goto _label))))))

(event `Reconnect_Event`
  ;[1 1 1] Reconnect Event
  (if (not (`self.ReconnectBlocker`))
    (set `self.ReconnectBlocker` true)
    (`PerceptionNeuronBPLibrary.NeuronDisconnect` self)
    (set `self.NeuronConnected` false)
    (bind _returnvalue (`PerceptionNeuronBPLibrary.NeuronConnect` self (`self.HostName`) (`self.Port`) (`self.EnableReferenceBone`) (`self.EnableDisplacement`) (`self.Motion Line Format`)))
    (set `self.NeuronConnected` _returnvalue)
    (set `self.ReconnectBlocker` false)))

(fn `UserConstructionScript`)